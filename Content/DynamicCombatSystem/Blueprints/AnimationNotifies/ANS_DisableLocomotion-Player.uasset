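; Animation notify state that blocks player locomotion for the duration of a montage or animation window, shown in the timeline as IgnoreLocomotion.
; On begin it casts the mesh owner to Symon_BP and clears AllowMovement; on end it sets AllowMovement back to true.
; It only affects Symon_BP owners and always re-enables movement rather than restoring the previous value.
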(fn ReceivedNotifyBegin
  (params (MeshComp :type Skeletal%20Mesh%20Component%20Object%20Reference) (Animation :type Anim%20Sequence%20Base%20Object%20Reference) (TotalDuration :type Float%20%28single-precision%29))
  (bind _assymon_bp (Utilities|Casting|CastToSymon_BP (Components|GetOwner MeshComp)))
  (bind _output_get (Variables|/Game/Characters/Symon/Symon_BP.Symon_BP_C|SetAllowMovement _assymon_bp false))
  (return _output_get))

(fn ReceivedNotifyEnd
  (params (MeshComp :type Skeletal%20Mesh%20Component%20Object%20Reference) (Animation :type Anim%20Sequence%20Base%20Object%20Reference))
  (bind _assymon_bp (Utilities|Casting|CastToSymon_BP (Components|GetOwner MeshComp)))
  (bind _output_get (Variables|/Game/Characters/Symon/Symon_BP.Symon_BP_C|SetAllowMovement _assymon_bp true))
  (return _output_get))

(fn GetNotifyName
  (return "IgnoreLocomotion"))