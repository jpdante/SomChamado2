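; Blueprint that links several levers (Alavancas) to one door (Porta), opening it only when all of them are active at once.
; On BeginPlay it binds its handler to each lever's state-change event.
; Each change recomputes Active as the AND of every lever's state and calls OpenDoorEvent on the door when true.
; It never closes the door again.
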(event Custom|OnChangeState
  (Variables|Default|SetActive true)
  (for _array_element (Variables|Default|GetAlavancas)
    (Variables|Default|SetActive (and (Variables|Default|GetActive) (Variables|/Game/Blueprints/Interact/Alavanca.Alavanca_C|GetActive _array_element))))
  (if (Variables|Default|GetActive)
    (Default|OpenDoorEvent (Variables|Default|GetPorta))))

(event EventBeginPlay
  (for _array_element (Variables|Default|GetAlavancas)
    (EventDispatchers|BindEventtoChangeState _array_element (delegate Custom|OnChangeState))))

(fn ConstructionScript)