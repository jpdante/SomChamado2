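; SavePoint is an interactable checkpoint that saves the player's progress.
; On interact, it builds a SaveDB object with the level name, inventory, health, arrow transform and teleport flag, then writes it to a single fixed slot.
; A successful save lights a blue torch effect and briefly shows a "Jogo Salvo" notification; a Saving flag blocks repeats, but stays set if saving fails.
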(event Custom|OnInteractEvent
  (params (Character :type Symon%20BP%20Object%20Reference))
  (bind _arrow (Variables|Default|GetArrow))
  (bind _health (Variables|/Game/Characters/Symon/Symon_BP.Symon_BP_C|GetHealth Character))
  (if (not (Variables|Default|GetSaving))
    (Variables|Default|SetSaving true)
    (bind _returnvalue (Game|ConstructObjectfromClass "/Game/Blueprints/Models/SaveDB.SaveDB_C" (Game|GetPlayerController 0)))
    (bind _returnvalue_2 (Game|GetCurrentLevelName true))
    (Variables|/Game/Blueprints/Models/SaveDB.SaveDB_C|SetCurrentLevel _returnvalue (Utilities|String|StringToName _returnvalue_2))
    (Variables|/Game/Blueprints/Models/SaveDB.SaveDB_C|SetInventory _returnvalue (Variables|/Game/Characters/Symon/Symon_BP.Symon_BP_C|GetInventory Character))
    (Variables|/Game/Blueprints/Models/SaveDB.SaveDB_C|SetMaxHealth _returnvalue (Variables|/Game/DynamicCombatSystem/Blueprints/ActorComponents/BPC_StatisticComponent.BPC_StatisticComponent_C|GetMaxValue _health))
    (Variables|/Game/Blueprints/Models/SaveDB.SaveDB_C|SetCurrentHealth _returnvalue (Default|GetCurrentValue _health))
    (Variables|/Game/Blueprints/Models/SaveDB.SaveDB_C|SetLocation _returnvalue (Transformation|GetWorldLocation _arrow))
    (Variables|/Game/Blueprints/Models/SaveDB.SaveDB_C|SetRotation _returnvalue (Transformation|GetWorldRotation _arrow))
    (Variables|/Game/Blueprints/Models/SaveDB.SaveDB_C|SetAllowTeleport _returnvalue (Variables|Default|GetAllowTeleport))
    (|Save _returnvalue)))

(event EventBeginPlay
  (EventDispatchers|BindEventtoOnInteract (delegate Custom|OnInteractEvent)))

(fn ConstructionScript)