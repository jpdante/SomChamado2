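; Collectable world pickup that the player interacts with to collect keys, crafting materials, puzzle pieces and other items.
; The construction script picks the mesh from Item.ItemType and sets the callout particle's visibility.
; On interact, it adds the item to the Character, or raises max health for Boost Vida, then plays a sound and destroys itself.
; Livro has no mesh case, and Energetico has a mesh but no interact handling.
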(event Custom|OnInteractEvent
  (params (Character :type Symon%20BP%20Object%20Reference))
  (bind _health (Variables|/Game/Characters/Symon/Symon_BP.Symon_BP_C|GetHealth Character))
  (bind _item (Variables|Item|GetItem))
  (switch Utilities|FlowControl|Switch|SwitchonItemsEnum (.ItemType (Utilities|Struct|BreakSuperItem _item))
    (:NewEnumerator0
      (Default|AddItem Character _item :!label _label))
    (:NewEnumerator1
      (Variables|/Game/DynamicCombatSystem/Blueprints/ActorComponents/BPC_StatisticComponent.BPC_StatisticComponent_C|SetMaxValue _health (+ (Variables|/Game/DynamicCombatSystem/Blueprints/ActorComponents/BPC_StatisticComponent.BPC_StatisticComponent_C|GetMaxValue _health) 25.0)))
    (:NewEnumerator2
      (goto _label))
    (:NewEnumerator5
      (goto _label))
    (:NewEnumerator6
      (goto _label))
    (:NewEnumerator7
      (goto _label))
    (:NewEnumerator9
      (goto _label))
    (:NewEnumerator10
      (goto _label))
    (:NewEnumerator11
      (goto _label))
    (:NewEnumerator12
      (goto _label))
    (:NewEnumerator13
      (goto _label))
    (:NewEnumerator14
      (goto _label))
    (:NewEnumerator15
      (goto _label))
    (:NewEnumerator16
      (goto _label)))
  (Audio|PlaySound2D "/Game/Assets/Sound/PegarItem.PegarItem" 1.0 1.0 0.0 0 0)
  (Actor|DestroyActor))

(event EventBeginPlay
  (|CallParentFunction)
  (EventDispatchers|BindEventtoOnInteract (delegate Custom|OnInteractEvent)))

(event Collision|EventActorBeginOverlap
  (params (OtherActor :type Actor%20Object%20Reference))
  (|CallParentFunction OtherActor) ; This node is disabled and will not be called.\nDrag off pins to build functionality.
)

(event EventTick
  (params (DeltaSeconds :type Float%20%28single-precision%29))
  (|CallParentFunction DeltaSeconds) ; This node is disabled and will not be called.\nDrag off pins to build functionality.
)

(fn ConstructionScript
  (bind _staticmesh (Variables|Default|GetStaticMesh))
  (|CallParentFunction)
  (Rendering|SetVisibility (Variables|Default|GetP_TreasureChest_CallOut_loop_Tier1) (Variables|Default|GetVisibility) false)
  (switch Utilities|FlowControl|Switch|SwitchonItemsEnum (.ItemType (Utilities|Struct|BreakSuperItem (Variables|Item|GetItem)))
    (:NewEnumerator0
      (Components|StaticMesh|SetStaticMesh _staticmesh "/Game/Blueprints/Interact/Mesh/chave.chave"))
    (:NewEnumerator1
      (Components|StaticMesh|SetStaticMesh _staticmesh "/Game/Blueprints/Interact/Mesh/Boost.Boost"))
    (:NewEnumerator2
      (Components|StaticMesh|SetStaticMesh _staticmesh "/Game/Blueprints/Interact/Mesh/Medkit1.Medkit1"))
    (:NewEnumerator5
      (Components|StaticMesh|SetStaticMesh _staticmesh "/Game/ForestSet/Coletaveis/Mato_Planta.Mato_Planta"))
    (:NewEnumerator6
      (Components|StaticMesh|SetStaticMesh _staticmesh "/Game/Blueprints/Interact/Mesh/ferro.ferro"))
    (:NewEnumerator9
      (Components|StaticMesh|SetStaticMesh _staticmesh "/Game/Levels/Tutorial/Assets/Pecas_Final_Tutorial_Peca_B.Pecas_Final_Tutorial_Peca_B"))
    (:NewEnumerator10
      (Components|StaticMesh|SetStaticMesh _staticmesh "/Game/Levels/Tutorial/Assets/Pecas_Final_Tutorial_Peca_B1.Pecas_Final_Tutorial_Peca_B1"))
    (:NewEnumerator11
      (Components|StaticMesh|SetStaticMesh _staticmesh "/Game/Levels/Tutorial/Assets/Pecas_Final_Tutorial_polySurface9.Pecas_Final_Tutorial_polySurface9"))
    (:NewEnumerator12
      (Components|StaticMesh|SetStaticMesh _staticmesh "/Game/Levels/Tutorial/Assets/Pedaco_Mosaico.Pedaco_Mosaico"))
    (:NewEnumerator13
      (Components|StaticMesh|SetStaticMesh _staticmesh "/Game/MultistoryDungeons/Meshes/Props/Bottle_01.Bottle_01"))
    (:NewEnumerator14
      (Components|StaticMesh|SetStaticMesh _staticmesh "/Game/Levels/OpenWorld/Cenario3/Backup_Mosaico_Quebrado_P_MosaicoQebrado1.Backup_Mosaico_Quebrado_P_MosaicoQebrado1"))
    (:NewEnumerator15
      (Components|StaticMesh|SetStaticMesh _staticmesh "/Game/Levels/OpenWorld/Cenario3/Backup_Mosaico_Quebrado_P_MosaicoQebrado2.Backup_Mosaico_Quebrado_P_MosaicoQebrado2"))
    (:NewEnumerator16
      (Components|StaticMesh|SetStaticMesh _staticmesh "/Game/Levels/OpenWorld/Cenario3/Backup_Mosaico_Quebrado_P_MosaicoQebrado3.Backup_Mosaico_Quebrado_P_MosaicoQebrado3"))
    (:NewEnumerator17
      (Components|StaticMesh|SetStaticMesh _staticmesh "/Game/MultistoryDungeons/Meshes/Props/Bottle_03.Bottle_03"))))