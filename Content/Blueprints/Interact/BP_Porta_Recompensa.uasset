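; Reward door actor that swings its mesh open or closed through Open, Close and Toggle events.
; A Mirror flag picks between two yaw timelines, played to open and reversed to close.
; When the timeline finishes, it can load a named level if TeleportToLevel is set.
; The interact handler bound on BeginPlay is empty, and the item check before opening is disconnected.
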(event Custom|OpenDoor_Event
  (if (Variables|Default|GetMirror)
    (Variables|Default|SetIsOpen true)
    (bind _doorrotation (Timeline|DoorAnimMirror Play)
      (:Update
        (Transformation|SetRelativeRotation (Variables|Default|GetStaticMesh) (Math|Rotator|MakeRotator 0.0 0.0 _doorrotation) false false))
      (:Finished
        (if (Variables|Default|GetTeleportToLevel) :!label _label
          (Game|OpenLevel(byName) (Variables|Default|GetLevelName)))))
    (else
      (Variables|Default|SetIsOpen true)
      (bind _doorrotation_2 (Timeline|DoorAnim Play)
        (:Update
          (Transformation|SetRelativeRotation (Variables|Default|GetStaticMesh) (Math|Rotator|MakeRotator 0.0 0.0 _doorrotation_2) false false))
        (:Finished
          (goto _label))))))

(event Custom|CloseDoor_Event
  (if (Variables|Default|GetMirror)
    (Variables|Default|SetIsOpen false)
    (bind _doorrotation (Timeline|DoorAnimMirror Reverse)
      (:Update
        (Transformation|SetRelativeRotation (Variables|Default|GetStaticMesh) (Math|Rotator|MakeRotator 0.0 0.0 _doorrotation) false false))
      (:Finished
        (if (Variables|Default|GetTeleportToLevel) :!label _label
          (Game|OpenLevel(byName) (Variables|Default|GetLevelName)))))
    (else
      (Variables|Default|SetIsOpen false)
      (bind _doorrotation_2 (Timeline|DoorAnim Reverse)
        (:Update
          (Transformation|SetRelativeRotation (Variables|Default|GetStaticMesh) (Math|Rotator|MakeRotator 0.0 0.0 _doorrotation_2) false false))
        (:Finished
          (goto _label))))))

(event Custom|ToggleDoor_Event
  (bind _mirror (Variables|Default|GetMirror))
  (if (not (Variables|Default|GetIsOpen))
    (if _mirror
      (Variables|Default|SetIsOpen true)
      (bind _doorrotation (Timeline|DoorAnimMirror Play)
        (:Update
          (Transformation|SetRelativeRotation (Variables|Default|GetStaticMesh) (Math|Rotator|MakeRotator 0.0 0.0 _doorrotation) false false))
        (:Finished
          (if (Variables|Default|GetTeleportToLevel) :!label _label
            (Game|OpenLevel(byName) (Variables|Default|GetLevelName)))))
      (else
        (Variables|Default|SetIsOpen true)
        (bind _doorrotation_2 (Timeline|DoorAnim Play)
          (:Update
            (Transformation|SetRelativeRotation (Variables|Default|GetStaticMesh) (Math|Rotator|MakeRotator 0.0 0.0 _doorrotation_2) false false))
          (:Finished
            (goto _label)))))
    (elif _mirror
      (Variables|Default|SetIsOpen false)
      (Timeline|DoorAnimMirror Reverse)
      (else
        (Variables|Default|SetIsOpen false)
        (Timeline|DoorAnim Reverse)))))

(event Custom|CustomEvent_0
  (params (Character :type Symon%20BP%20Object%20Reference)))

(event EventBeginPlay
  (EventDispatchers|BindEventtoOnInteract (delegate Custom|CustomEvent_0)))

(event Collision|EventActorBeginOverlap
  (params (OtherActor :type Actor%20Object%20Reference)))

(event EventTick
  (params (DeltaSeconds :type Float%20%28single-precision%29)))

(fn ConstructionScript)