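; Interactable torch pillar whose blue fire effect toggles on and off when a character interacts with it.
; BeginPlay binds the interact event, which flips the Activated flag and calls UpdateParticle to set the fire particle's visibility to match.
; The construction script calls the same function, so the flame reflects the initial Activated state.
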(event Custom|OnInteractEvent
  (params (Character :type Symon%20BP%20Object%20Reference))
  (if (Variables|Default|GetActivated)
    (Variables|Default|SetActivated false)
    (else
      (Variables|Default|SetActivated true)))
  (CallFunction|UpdateParticle))

(event EventBeginPlay
  (EventDispatchers|BindEventtoOnInteract (delegate Custom|OnInteractEvent)))

(fn ConstructionScript
  (CallFunction|UpdateParticle))

(fn UpdateParticle
  (Rendering|SetVisibility (Variables|Default|GetP_Fire_Torch_Blue) (Variables|Default|GetActivated) false))