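; BookInteract is an interactable book that shows a timed text overlay when a character interacts with it.
; It binds to its OnInteract event on BeginPlay, then creates a BookHud widget for player controller 0 and sets the book's Text on it.
; The widget is hidden after a configurable delay and removed shortly afterward, while a Triggered flag blocks repeat interactions until the sequence ends.
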(event Custom|OnInteractEvent
  (params (Character :type BP%20Combat%20Character%20Object%20Reference))
  (if (not (Variables|Default|GetTriggered))
    (Variables|Default|SetTriggered true)
    (bind _returnvalue (UserInterface|CreateWidget "/Game/Blueprints/UI/InGame/BookHud.BookHud_C" (Game|GetPlayerController 0)))
    (UserInterface|Viewport|AddtoViewport _returnvalue 0)
    (Default|SetText _returnvalue (Variables|Default|GetText))
    (Default|ShoworHide _returnvalue true)
    (Utilities|FlowControl|Delay (Variables|Default|GetDelay))
    (Default|ShoworHide _returnvalue false)
    (Utilities|FlowControl|Delay 2.0)
    (Widget|RemovefromParent _returnvalue)
    (Variables|Default|SetTriggered false)))

(event EventBeginPlay
  (|CallParentFunction)
  (EventDispatchers|BindEventtoOnInteract (delegate Custom|OnInteractEvent)))

(event Collision|EventActorBeginOverlap
  (params (OtherActor :type Actor%20Object%20Reference))
  (|CallParentFunction OtherActor) ; This node is disabled and will not be called.\nDrag off pins to build functionality.
)

(event EventTick
  (params (DeltaSeconds :type Float%20%28single-precision%29))
  (|CallParentFunction DeltaSeconds) ; This node is disabled and will not be called.\nDrag off pins to build functionality.
)

(fn ConstructionScript
  (|CallParentFunction))