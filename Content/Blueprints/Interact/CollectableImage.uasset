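; Interactable collectable actor that gives the interacting character an item and shows an associated image on screen.
; The construction script picks the static mesh from the item type, covering keys, puzzle pieces, health, herbs, iron and books.
; On interaction it adds the configured type and quantity to the character, destroys itself, then opens a CollectableImage widget for the first player controller and initializes it with its image.
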(event Custom|OnInteractEvent
  (params (Character :type BP%20Combat%20Character%20Object%20Reference))
  (Default|AddItem Character (Variables|Item|GetItemType) (Variables|Item|GetQuantity))
  (Actor|DestroyActor)
  (bind _returnvalue (UserInterface|CreateWidget "/Game/Blueprints/UI/InGame/CollectableImage.CollectableImage_C" (Game|GetPlayerController 0)))
  (UserInterface|Viewport|AddtoViewport _returnvalue 0)
  (Default|Init _returnvalue (Variables|Item|GetImage)))

(event EventBeginPlay
  (|CallParentFunction)
  (EventDispatchers|BindEventtoOnInteract (delegate Custom|OnInteractEvent)))

(event Collision|EventActorBeginOverlap
  (params (OtherActor :type Actor%20Object%20Reference))
  (|CallParentFunction OtherActor) ; This node is disabled and will not be called.\nDrag off pins to build functionality.
)

(event EventTick
  (params (DeltaSeconds :type Float%20%28single-precision%29))
  (|CallParentFunction DeltaSeconds) ; This node is disabled and will not be called.\nDrag off pins to build functionality.
)

(fn ConstructionScript
  (bind _staticmesh (Variables|Default|GetStaticMesh))
  (|CallParentFunction)
  (switch Utilities|FlowControl|Switch|SwitchonItemsEnum (Variables|Item|GetItemType)
    (:NewEnumerator0
      (Components|StaticMesh|SetStaticMesh _staticmesh "/Game/Blueprints/Interact/Mesh/chave.chave"))
    (:NewEnumerator1
      (Components|StaticMesh|SetStaticMesh _staticmesh "/Game/Blueprints/Interact/Mesh/Boost.Boost"))
    (:NewEnumerator2
      (Components|StaticMesh|SetStaticMesh _staticmesh "/Game/Blueprints/Interact/Mesh/Medkit1.Medkit1"))
    (:NewEnumerator5
      (Components|StaticMesh|SetStaticMesh _staticmesh "/Game/Blueprints/Interact/Mesh/Erva1.Erva1"))
    (:NewEnumerator6
      (Components|StaticMesh|SetStaticMesh _staticmesh "/Game/Blueprints/Interact/Mesh/ferro.ferro"))
    (:NewEnumerator7
      (Components|StaticMesh|SetStaticMesh _staticmesh "/Game/Levels/Level1/Assets/Livro_Livro1.Livro_Livro1"))))