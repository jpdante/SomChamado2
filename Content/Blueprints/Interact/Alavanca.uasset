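; Interactable lever (Alavanca) that toggles between active and inactive when a character interacts with it.
; It binds to OnInteract on BeginPlay, then flips Active and plays or reverses a timeline that drives the lever mesh's roll.
; AllowToggle blocks further input during the animation; when the timeline finishes, it re-enables toggling and calls ChangeState.
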(event Custom|CustomEvent_0
  (params (Character :type Symon%20BP%20Object%20Reference))
  (if (Variables|Default|GetAllowToggle)
    (Variables|Default|SetAllowToggle false)
    (if (Variables|Default|GetActive)
      (Variables|Default|SetActive false)
      (bind _curve (Timeline|Timeline_0 Reverse)
        (:Update
          (Transformation|SetRelativeRotation (Variables|Default|GetAlavanca_Alavanca) (Math|Rotator|MakeRotator _curve 0.0 0.0) false false))
        (:Finished
          (Variables|Default|SetAllowToggle true)
          (Default|CallChangeState)))
      (else
        (Variables|Default|SetActive true)
        (Timeline|Timeline_0 Play)))))

(event EventBeginPlay
  (EventDispatchers|BindEventtoOnInteract (delegate Custom|CustomEvent_0)))

(event Collision|EventActorBeginOverlap
  (params (OtherActor :type Actor%20Object%20Reference)))

(event EventTick
  (params (DeltaSeconds :type Float%20%28single-precision%29)))

(fn ConstructionScript
  (|CallParentFunction))