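; NotificationBox is a one-shot trigger volume that shows an on-screen notification when its collision component is first overlapped.
; The overlap creates a NotificationHud widget for player 0, sets its text and color from the box's variables with "\n" sequences stripped, and shows it.
; After a configurable delay it hides the widget, waits briefly, then removes it and destroys itself.
; The overlapping actor is not filtered.
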(event OnComponentBeginOverlap(CollisionComponent)
  (params (OverlappedComponent :type Primitive%20Component%20Object%20Reference) (OtherActor :type Actor%20Object%20Reference) (OtherComp :type Primitive%20Component%20Object%20Reference) (OtherBodyIndex :type Integer) (bFromSweep :type Boolean) (SweepResult :type Hit%20Result%20Structure%20%28by%20ref%29))
  (if (not (Variables|Default|GetTriggered))
    (Variables|Default|SetTriggered true)
    (bind _returnvalue (UserInterface|CreateWidget "/Game/Blueprints/UI/InGame/NotificationHud.NotificationHud_C" (Game|GetPlayerController 0)))
    (UserInterface|Viewport|AddtoViewport _returnvalue 0)
    (Default|SetTextEvent _returnvalue (Utilities|Text|ToText(String) (Utilities|String|Replace (Variables|Trigger|GetNotificationText) "\\n" " 
")) (Variables|Trigger|GetNotificationColor))
    (Default|ShowEvent _returnvalue)
    (Utilities|FlowControl|Delay (Variables|Trigger|GetDelay))
    (Default|HideEvent _returnvalue)
    (Utilities|FlowControl|Delay 1.0)
    (Widget|RemovefromParent _returnvalue)
    (Class|JavascriptTestLibrary|DestroyUObject _returnvalue)
    (Actor|DestroyActor self)))

(event EventBeginPlay)

(event Collision|EventActorBeginOverlap
  (params (OtherActor :type Actor%20Object%20Reference)))

(event EventTick
  (params (DeltaSeconds :type Float%20%28single-precision%29)))

(fn ConstructionScript)